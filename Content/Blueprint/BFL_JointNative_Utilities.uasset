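; Blueprint function library for Joint participants that finds an actor's components of a given class matching participant gameplay tags.
; Components opt in through the QueryableWithParticipantTag interface, which supplies their tag container for a non-exact any-match test.
; One lookup takes an owner and tag container directly.
; The other derives both from a participant component after validity checks.
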(fn `GetComponentsForParitipantWithParticipantComponent`
  (params (ParticipantComponent :type "DialogueParticipantComponent Object Reference") (`Component Class` :type "ActorComponent Class Reference"))
  (returns (FoundComponents :type "Array of ActorComponent Object Reference"))
  (locals (NewLocalVar_0 :type "Array of ActorComponent Object Reference"))
  (bind _returnvalue (`ActorComponent.GetOwner` ParticipantComponent))
  (bind _newlocalvar_0 (`local.NewLocalVar_0`))
  (`/Engine/EditorBlueprintResources/StandardMacros.IsValid` ParticipantComponent
    (:`Is Valid`
      (`/Engine/EditorBlueprintResources/StandardMacros.IsValid` _returnvalue
        (:`Is Valid`
          (`KismetArrayLibrary.Array_Clear` _newlocalvar_0)
          (`|ExecutionSequence`
            (:`then_0`
              (for _array_element (`Actor.K2_GetComponentsByClass` _returnvalue `Component Class`)
                (bind _asbp_joint_component_queryable_with_participant_tag_interface (cast `/JointNative/Blueprint/BP_Joint_Component_QueryableWithParticipantTagInterface` _array_element))
                (bind _participant_tag_container (`/JointNative/Blueprint/BP_Joint_Component_QueryableWithParticipantTagInterface.Interface_ProvideParticipantTagContainer` _asbp_joint_component_queryable_with_participant_tag_interface))
                (if (`BlueprintGameplayTagLibrary.HasAnyTags` _participant_tag_container (`DialogueParticipantComponent.ParticipantTag` ParticipantComponent))
                  (`KismetArrayLibrary.Array_Add` (`local.NewLocalVar_0`) _array_element))))
            (:`then_1`
              (return _newlocalvar_0))))))))

(fn `GetComponentsForParitipantWithParticipantTag`
  (params (Owner :type "Actor Object Reference") (`Component Class` :type "ActorComponent Class Reference") (TagContainer :type "GameplayTagContainer Structure"))
  (returns (FoundComponents :type "Array of ActorComponent Object Reference"))
  (locals (NewLocalVar_0 :type "Array of ActorComponent Object Reference"))
  (bind _newlocalvar_0 (`local.NewLocalVar_0`))
  (`KismetArrayLibrary.Array_Clear` _newlocalvar_0)
  (`|ExecutionSequence`
    (:`then_0`
      (for _array_element (`Actor.K2_GetComponentsByClass` Owner `Component Class`)
        (bind _asbp_joint_component_queryable_with_participant_tag_interface (cast `/JointNative/Blueprint/BP_Joint_Component_QueryableWithParticipantTagInterface` _array_element))
        (bind _participant_tag_container (`/JointNative/Blueprint/BP_Joint_Component_QueryableWithParticipantTagInterface.Interface_ProvideParticipantTagContainer` _asbp_joint_component_queryable_with_participant_tag_interface))
        (if (`BlueprintGameplayTagLibrary.HasAnyTags` _participant_tag_container TagContainer)
          (`KismetArrayLibrary.Array_Add` (`local.NewLocalVar_0`) _array_element))))
    (:`then_1`
      (return _newlocalvar_0))))